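; BP_Trap_Slip is a slip trap that speeds up the first-person character while it stands inside the trap's sphere.
; Sphere begin overlap casts to BP_FirstPersonCharacter, raises its max walk speed and prints a debug message.
; End overlap sets the speed to a fixed lower value instead of restoring a saved one.
; An empty Slow event and unconnected timer and overlap-query nodes do nothing.
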(event `self.Sphere.OnComponentBeginOverlap`
  (params (OverlappedComponent :type "PrimitiveComponent Object Reference") (OtherActor :type "Actor Object Reference") (OtherComp :type "PrimitiveComponent Object Reference") (OtherBodyIndex :type Integer) (bFromSweep :type Boolean) (SweepResult :type "HitResult Structure (by ref)"))
  (bind _asbp_first_person_character (cast `/Game/FirstPerson/Blueprints/BP_FirstPersonCharacter` OtherActor))
  (set `CharacterMovementComponent.MaxWalkSpeed` 1500.0 (`Character.CharacterMovement` _asbp_first_person_character))
  (`KismetSystemLibrary.PrintString` "Hello"))

(event `self.ReceiveBeginPlay`)

(event `Slow`)

(event `self.Sphere.OnComponentEndOverlap`
  (params (OverlappedComponent :type "PrimitiveComponent Object Reference") (OtherActor :type "Actor Object Reference") (OtherComp :type "PrimitiveComponent Object Reference") (OtherBodyIndex :type Integer))
  (bind _asbp_first_person_character (cast `/Game/FirstPerson/Blueprints/BP_FirstPersonCharacter` OtherActor))
  (set `CharacterMovementComponent.MaxWalkSpeed` 600.0 (`Character.CharacterMovement` _asbp_first_person_character)))

(fn `UserConstructionScript`)