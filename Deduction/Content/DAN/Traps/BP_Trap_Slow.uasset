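; BP_Trap_Slow is a trap that slows first-person characters inside its sphere.
; A looping one-second timer finds overlapping characters and cuts their max walk speed in steps, clamped to a minimum, printing a debug message each time.
; Leaving the sphere resets speed to a hard-coded default rather than the character's original value.
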(event `self.ReceiveBeginPlay`
  (`KismetSystemLibrary.K2_SetTimerDelegate` (delegate `Slow`) 1.0 true))

(event `Slow`
  (for _array_element (`PrimitiveComponent.GetOverlappingActors` (`self.Sphere`) "/Game/FirstPerson/Blueprints/BP_FirstPersonCharacter.BP_FirstPersonCharacter_C")
    (bind _asbp_first_person_character (cast `/Game/FirstPerson/Blueprints/BP_FirstPersonCharacter` _array_element))
    (bind _charactermovement (`Character.CharacterMovement` _asbp_first_person_character))
    (set `CharacterMovementComponent.MaxWalkSpeed` (`KismetMathLibrary.FClamp` (- (`CharacterMovementComponent.MaxWalkSpeed` _charactermovement) 200.0) 100.0 600.0) _charactermovement)
    (`KismetSystemLibrary.PrintString` "Hello")))

(event `self.Sphere.OnComponentEndOverlap`
  (params (OverlappedComponent :type "PrimitiveComponent Object Reference") (OtherActor :type "Actor Object Reference") (OtherComp :type "PrimitiveComponent Object Reference") (OtherBodyIndex :type Integer))
  (bind _asbp_first_person_character (cast `/Game/FirstPerson/Blueprints/BP_FirstPersonCharacter` OtherActor))
  (set `CharacterMovementComponent.MaxWalkSpeed` 600.0 (`Character.CharacterMovement` _asbp_first_person_character)))

(fn `UserConstructionScript`)