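; Trap actor that randomly teleports the first-person character when it overlaps the trap's sphere.
; The overlap casts to BP_FirstPersonCharacter, then teleports it to a random reachable navmesh point at a zeroed rotation.
; The search is centered on player 0's location rather than the trap, with a randomized radius, and its success is not checked.
; Disconnected slow-effect and timer logic remains in the graph and never runs.
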(event `self.Sphere.OnComponentBeginOverlap`
  (params (OverlappedComponent :type "PrimitiveComponent Object Reference") (OtherActor :type "Actor Object Reference") (OtherComp :type "PrimitiveComponent Object Reference") (OtherBodyIndex :type Integer) (bFromSweep :type Boolean) (SweepResult :type "HitResult Structure (by ref)"))
  (bind _asbp_first_person_character (cast `/Game/FirstPerson/Blueprints/BP_FirstPersonCharacter` OtherActor))
  (`self.K2_TeleportTo` :`self` _asbp_first_person_character :`DestLocation` (`NavigationSystemV1.K2_GetRandomReachablePointInRadius` (`self.K2_GetActorLocation` (`GameplayStatics.GetPlayerCharacter` 0)) (`KismetMathLibrary.RandomFloatInRange` 100.0 1000.0) null null)))

(event `self.ReceiveBeginPlay`)

(event `Slow`)

(fn `UserConstructionScript`)