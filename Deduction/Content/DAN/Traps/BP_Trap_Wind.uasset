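; Wind trap that slows the player character and pushes it along the wind direction.
; Entering the Box lowers walk speed and starts a fast looping timer; leaving restores speed but never clears the timer.
; Each tick of that timer sphere-traces forward from five arrow components, with debug drawing.
; Every trace hitting the player adds a velocity-change impulse along the first arrow's forward vector.
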(event `self.Box.OnComponentBeginOverlap`
  (params (OverlappedComponent :type "PrimitiveComponent Object Reference") (OtherActor :type "Actor Object Reference") (OtherComp :type "PrimitiveComponent Object Reference") (OtherBodyIndex :type Integer) (bFromSweep :type Boolean) (SweepResult :type "HitResult Structure (by ref)"))
  (if (== OtherActor (`GameplayStatics.GetPlayerCharacter` 0))
    (set `CharacterMovementComponent.MaxWalkSpeed` 250.0 (`self.GetComponentByClass` OtherActor "/Script/Engine.CharacterMovementComponent"))
    (`KismetSystemLibrary.K2_SetTimerDelegate` (delegate `Wind Push`) 0.03 true)))

(event `Wind Push`
  (for (_ _array_index) (`|MakeArray` (`self.Arrow`) (`self.Arrow1`) (`self.Arrow2`) (`self.Arrow3`) (`self.Arrow4`))
    (bind _returnvalue (select `int` _array_index :`0` (`self.Arrow`) :`1` (`self.Arrow1`) :`2` (`self.Arrow2`) :`3` (`self.Arrow3`) :`4` (`self.Arrow4`)))
    (bind _returnvalue_2 (`SceneComponent.K2_GetComponentLocation` _returnvalue))
    (bind (_outhit _returnvalue_3) (`KismetSystemLibrary.SphereTraceSingleForObjects` :`Start` _returnvalue_2 :`End` (+ _returnvalue_2 (* (`SceneComponent.GetForwardVector` _returnvalue) (`self.LIneExt`))) :`Radius` 20.0 :`ObjectTypes` (`|MakeArray` "ObjectTypeQuery1" "ObjectTypeQuery2" "ObjectTypeQuery3" "ObjectTypeQuery4" :!type "EObjectTypeQuery Enum") :`DrawDebugType` "ForDuration"))
    (bind (_bblockinghit _binitialoverlap _time _distance _location _impactpoint _normal _impactnormal _physmat _hitactor) (`GameplayStatics.BreakHitResult` _outhit))
    (if (and _returnvalue_3 (== _hitactor (`GameplayStatics.GetPlayerCharacter` 0)))
      (`CharacterMovementComponent.AddImpulse` (`self.GetComponentByClass` _hitactor "/Script/Engine.CharacterMovementComponent") (* (`SceneComponent.GetForwardVector` (`self.Arrow`)) 75.0) true))))

(event `self.Box.OnComponentEndOverlap`
  (params (OverlappedComponent :type "PrimitiveComponent Object Reference") (OtherActor :type "Actor Object Reference") (OtherComp :type "PrimitiveComponent Object Reference") (OtherBodyIndex :type Integer))
  (if (== OtherActor (`GameplayStatics.GetPlayerCharacter` 0))
    (set `CharacterMovementComponent.MaxWalkSpeed` 600.0 (`self.GetComponentByClass` OtherActor "/Script/Engine.CharacterMovementComponent"))))

(fn `UserConstructionScript`)