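; Level generation manager that builds a room layout scaled to player count, triggered on BeginPlay when enabled and relayed by server-to-client RPCs.
; A retry-capped macro picks random BP_RoomSpawnLocations, rolls weighted room classes by ring override and checks clearance before spawning.
; It then places doors at every location, locked where unused, and scatters sigil collectables over shuffled positions.
; A GameSeed-based random stream drives generation; older logic remains disconnected.
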(event `self.ReceiveBeginPlay`
  ;[0.1451 1 0.1373] Debug map generation call to test replication. TBF, could just be left on begin play
  (`|VariableSetRef` (`self.Random Stream`) (`KismetMathLibrary.MakeRandomStream` (`self.GameSeed`)))
  (if (`self.bEnabled`)
    (`KismetSystemLibrary.Delay` 1.0)
    (`self.RPC Server Start Generation` (`GameplayStatics.GetNumPlayerStates`))))

(event `RPC Server Generate Furniture`
  (params (InputPin :type "RandomStream Structure (by ref)"))
  (`self.RPC Client Generate Furniture` InputPin))

(event `RPC Client Generate Furniture`
  (params (InputPin :type "RandomStream Structure (by ref)"))
  (bind _outactors (`GameplayStatics.GetAllActorsOfClass` "/Game/Generation/BP_RoomTemplate.BP_RoomTemplate_C"))
  (for _ _outactors
    _))

(event `RPC Server Start Generation`
  (params (PlayerCount :type Integer))
  ;[0.1451 1 0.1373] Replication poopoo
  (`self.RPC Client Start Generation` PlayerCount))

(event `RPC Client Start Generation`
  (params (PlayerCount :type Integer))
  ;[0.1451 1 0.1373] Replication poopoo
  (`self.StartGeneration` PlayerCount))

(event `/Game/Generation/Interfaces/BPI_LevelGeneration.StartGeneration`
  (params (PlayerCount :type Integer))
  (bind _outactors (`GameplayStatics.GetAllActorsOfClass` "/Game/Generation/GenerationSetupComponents/BP_RoomSpawnLocation.BP_RoomSpawnLocation_C")) ; Get all Room Spawn Locations in level
  (bind _output_get (set `self.RoomSpawns` _outactors))
  (bind (_spawn_location_bp _transform_index _valid_room_class) (`self.Start Spawn Process` (+ (`self.RoomBaseCount`) (* (`self.RoomsPerPlayerCount`) PlayerCount)))
    (:`Next`
      (if (`KismetSystemLibrary.IsValidClass` _valid_room_class)
        (`/Game/Generation/GenerationSetupComponents/BP_RoomSpawnLocation.SetInUse` _spawn_location_bp true)
        (`|SpawnActorFromClass` _valid_room_class (`self.GetTransform` _spawn_location_bp) "Undefined" "MultiplyWithRoot" null true (`self.Random Stream`) (`self.Spawning Data`) null)
        (`/Engine/EditorBlueprintResources/StandardMacros.IncrementInt` (`self.RoomCount`))))
    (:`Completed`
      (for _array_element _output_get
        (bind _returnvalue (`|SpawnActorFromClass` "/Game/Generation/Furniture/BP_BedroomDoor.BP_BedroomDoor_C" (`self.GetTransform` _array_element) "Undefined" "MultiplyWithRoot" null false null)) ; Spawn a door here and mark it as openable (unlocked)
        (`/Game/Generation/Furniture/BP_BedroomDoor.Set Door Locked Status` _returnvalue (not (`/Game/Generation/GenerationSetupComponents/BP_RoomSpawnLocation.GetInUse` _array_element))))
      (bind _outactors_2 (`GameplayStatics.GetAllActorsOfClass` "/Game/Generation/GenerationSetupComponents/BP_SigilPosition.BP_SigilPosition_C")) ; Sigil Spawning
      (`KismetArrayLibrary.Array_ShuffleFromStream` _outactors_2 (`self.Random Stream`))
      (for _index (range 1 (+ (`KismetMathLibrary.Min` (`KismetArrayLibrary.Array_Length` _outactors_2) (+ (`self.SigilBaseCount`) (* (`self.SigilPerPlayerCount`) PlayerCount))) 1))
        (bind _returnvalue_2 (`|SpawnActorFromClass` "/Game/Inez/Sigil/BP_SigilCollectable.BP_SigilCollectable_C" (`self.GetTransform` (`|GetArrayItem` _outactors_2 (`self.Inline Decrement` _index))) "Undefined" "MultiplyWithRoot" null null))
        (`self.SetReplicates` _returnvalue_2 true)))))

(fn `CreateMapFromReplicatedArrays`
  (params (Array :type "Array of Name") (Array1 :type "Array of /Game/Generation/Data/F_BedroomEntryWeight Structure"))
  (returns (ReturnMap1 :type "Map of Name to /Game/Generation/Data/F_BedroomEntryWeight Structure"))
  (locals (ReturnMap :type "Map of Name to /Game/Generation/Data/F_BedroomEntryWeight Structure"))
  (bind _returnmap (`local.ReturnMap`))
  (`KismetSystemLibrary.PrintString` (`KismetStringLibrary.Concat_StrStr` "Length names: " (`KismetStringLibrary.Conv_IntToString` (`KismetArrayLibrary.Array_Length` Array))) true true (struct :`G` 0.66 :`B` 1.0 :`A` 1.0) 10.0)
  (`KismetSystemLibrary.PrintString` (`KismetStringLibrary.Concat_StrStr` "Length vals: " (`KismetStringLibrary.Conv_IntToString` (`KismetArrayLibrary.Array_Length` Array1))) true true (struct :`G` 0.66 :`B` 1.0 :`A` 1.0) 10.0)
  (for (_array_element _array_index) Array
    (`BlueprintMapLibrary.Map_Add` _returnmap _array_element (`|GetArrayItem` Array1 _array_index)))
  (return _returnmap))

(fn `GetWeightedItem`
  (params (FromDataTable :type "DataTable Object Reference"))
  (returns (`Selected Actor Class` :type "Actor Class Reference"))
  (return null))

(fn `SpawnNextRoom`
  (params (`At Transform` :type "Transform Structure"))
  (returns (Success :type Boolean) (Room :type "Actor Object Reference"))
  (bind _random_stream (`self.Random Stream`))
  (bind _selected_actor_class (`/Game/Generation/Data/BPFL_SharedFunctions.GetWeightedClass` :`Random Stream` _random_stream))
  (bind _returnvalue (`|SpawnActorFromClass` _selected_actor_class `At Transform` "Undefined" "MultiplyWithRoot" null null))
  (message `/Game/Generation/Interfaces/BPI_Room.PopulateFurniture` _returnvalue _random_stream (`|MakeMap` "None" :!type "Name" :!valuetype "/Game/Generation/Data/F_BedroomContentEntry Structure"))
  (bind _returnvalue_2 (`|SpawnActorFromClass` "/Game/Generation/Furniture/BP_BedroomDoor.BP_BedroomDoor_C" `At Transform` "Undefined" "MultiplyWithRoot" null false null)) ; Spawn a door here and mark it as openable (unlocked)
  (`/Game/Generation/Furniture/BP_BedroomDoor.Set Door Locked Status` _returnvalue_2 false)
  (return true _returnvalue))

(fn `UserConstructionScript`)