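; Level generation manager, marked OLD, that procedurally builds a hallway-and-bedroom layout from a seeded random stream.
; It spawns hallways left and right of a start room, gathering their room connection transforms.
; A capped loop macro picks random clearance-checked transforms, spawning weighted-random furnished bedrooms with unlocked doors, then locked doors on leftovers.
; Server-to-client RPCs relay generation and room spawns, with debug prints showing replication is being tested.
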(event `self.ReceiveBeginPlay`
  ;[0.1451 1 0.1373] Debug map generation call to test replication. TBF, could just be left on begin play
  (`|VariableSetRef` (`self.Random Stream`) (`KismetMathLibrary.MakeRandomStream` (`self.GameSeed`)))
  (if (`self.bEnabled`)
    (`self.RPC Server Start Generation` (`GameplayStatics.GetNumPlayerStates`))))

(event `RPC Server Start Generation`
  (params (PlayerCount :type Integer))
  ;[0.1451 1 0.1373] Replication poopoo
  (`self.RPC Client Start Generation` PlayerCount))

(event `RPC Client Start Generation`
  (params (PlayerCount :type Integer))
  ;[0.1451 1 0.1373] Replication poopoo
  (`self.StartGeneration` PlayerCount))

(event `/Game/Generation/Interfaces/BPI_LevelGeneration.StartGeneration`
  (params (PlayerCount :type Integer))
  (bind _startroom (`self.StartRoom`))
  ;[0.1451 1 0.1373] Start room generation by creating hallways off of start room
  (`/Engine/EditorBlueprintResources/StandardMacros.IsValid` _startroom
    (:`Is Valid`
      (bind (_world_left _world_right) (`/Game/Generation/BP_StartRoom.GetHallPoints` _startroom))
      (`self.SpawnHallwaySection` _world_left)
      (`self.SpawnHallwaySection` _world_right)
      (`self.Spawn Rooms` PlayerCount))
    (:`Is Not Valid`
      (`KismetSystemLibrary.PrintString` "Start room missing"))))

(event `SpawnHallwaySection`
  (params (`At Transform` :type "Transform Structure"))
  ;[0.1451 1 0.1373] Spawns a hallway at the given WORLD transform, adds to the Hallways array so can be iterated later for bedroom spawning
  (bind _returnvalue (`|SpawnActorFromClass` "/Game/Generation/Rooms/Preset/BP_Hallway.BP_Hallway_C" `At Transform` "AlwaysSpawn" "MultiplyWithRoot" null true null)) ; Spawn hallway. Transform is irrelevant cuz it gets overwritten immediately anyway
  (message `/Game/Generation/Interfaces/BPI_Room.SetOrigin` _returnvalue (`/Game/Generation/Rooms/Preset/BP_Hallway.Get Hall Points` _returnvalue))
  (`self.K2_SetActorTransform` _returnvalue `At Transform` false false)
  (`KismetArrayLibrary.Array_Add` (`self.Hallways`) null)
  (bind _point_transforms (message `/Game/Generation/Interfaces/BPI_Room.GetRoomConnectionPoints` _returnvalue))
  (`KismetArrayLibrary.Array_Append` (`self.HallwayRoomSpawnableTransforms`) _point_transforms)
  (message `/Game/Generation/Interfaces/BPI_Room.PopulateFurniture` _returnvalue (`self.Random Stream`)))

(event `Spawn Rooms`
  (params (`Player Count` :type Integer))
  (bind _hallwayroomspawnabletransforms (`self.HallwayRoomSpawnableTransforms`))
  ;[0.1451 1 0.1373] Room Spawning - Spawns rooms at random possible locations outlined in the Hallway BPs
  (if (`self.bIsDebug`)
    (`/Game/Generation/Data/BPFL_SharedFunctions.PrintArrayTransforms` (`self.HallwayRoomSpawnableTransforms`) true true true true (struct :`R` 1.0 :`G` 0.429656 :`B` 0.949287 :`A` 1.0) 0.5))
  (bind (_transform _transform_index) (`self.Start Spawn Process`) ; Effectively a fancy while loop with safeguards and inf loop protection
    (:`Next`
      (`self.RPC Server Spawn Next Room` _transform _transform_index)
      (`KismetSystemLibrary.PrintString` "Hello" true true (struct :`R` 0.805938 :`G` 1.0 :`A` 1.0)))
    (:`Completed`
      (if (> (`KismetArrayLibrary.Array_Length` _hallwayroomspawnabletransforms) 0)
        (for _array_element _hallwayroomspawnabletransforms
          (bind _returnvalue (`|SpawnActorFromClass` "/Game/Generation/Furniture/BP_BedroomDoor.BP_BedroomDoor_C" _array_element "Undefined" "MultiplyWithRoot" null null)) ; Spawn a door here and mark it as locked
          (`/Game/Generation/Furniture/BP_BedroomDoor.Set Door Locked Status` _returnvalue true)))
      (`KismetSystemLibrary.PrintString` "Generated"))))

(event `RPC Server Spawn Next Room`
  (params (`At Transform` :type "Transform Structure (by ref)") (`Transform Index` :type Integer))
  ;[0.1451 1 0.1373] Room Spawning - Spawns rooms at random possible locations outlined in the Hallway BPs
  (`self.RPC Client Spawn Next Room` `At Transform` `Transform Index`)
  (`KismetSystemLibrary.PrintString` "Server ran spawn room?" true true (struct :`G` 0.66 :`B` 1.0 :`A` 1.0) 2.0 "SRVER"))

(event `RPC Client Spawn Next Room`
  (params (`At Transform` :type "Transform Structure (by ref)") (`Transform Index` :type Integer))
  ;[0.1451 1 0.1373] Room Spawning - Spawns rooms at random possible locations outlined in the Hallway BPs
  (bind _success (`self.SpawnNextRoom` `At Transform`))
  (if _success
    (`/Engine/EditorBlueprintResources/StandardMacros.IncrementInt` (`self.RoomCount`)
      (:`  `
        (`KismetArrayLibrary.Array_RemoveItem` (`self.HallwayRoomSpawnableTransforms`) `At Transform`)
        (`KismetSystemLibrary.PrintString` "Client ran spawn room?" true true (struct :`R` 1.0 :`B` 0.306638 :`A` 1.0) 43434.0 "CLIENT")))
    (else
      (`KismetSystemLibrary.PrintString` "your mum yeah" true true (struct :`R` 1.0 :`B` 0.306638 :`A` 1.0) 43434.0 "CLIENT"))))

(fn `GetWeightedItem`
  (params (FromDataTable :type "DataTable Object Reference"))
  (returns (`Selected Actor Class` :type "Actor Class Reference"))
  (return null))

(fn `SpawnNextRoom`
  (params (`At Transform` :type "Transform Structure"))
  (returns (Success :type Boolean) (Room :type "Actor Object Reference"))
  (bind _random_stream (`self.Random Stream`))
  (bind _selected_actor_class (`/Game/Generation/Data/BPFL_SharedFunctions.GetWeightedClass` (`self.BedroomSpawnChances`) _random_stream))
  (bind _returnvalue (`|SpawnActorFromClass` _selected_actor_class `At Transform` "Undefined" "MultiplyWithRoot" null null))
  (message `/Game/Generation/Interfaces/BPI_Room.PopulateFurniture` _returnvalue _random_stream)
  (bind _returnvalue_2 (`|SpawnActorFromClass` "/Game/Generation/Furniture/BP_BedroomDoor.BP_BedroomDoor_C" `At Transform` "Undefined" "MultiplyWithRoot" null null)) ; Spawn a door here and mark it as openable (unlocked)
  (`/Game/Generation/Furniture/BP_BedroomDoor.Set Door Locked Status` _returnvalue_2 false)
  (return true _returnvalue))

(fn `UserConstructionScript`)