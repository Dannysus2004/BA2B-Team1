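; BP_Hallway is a hallway piece in the game's generation system, exposing the points where other pieces connect.
; GetHallPoints returns its OriginPoint and NextPoint as the hall's origin and next points.
; GetRoomConnectionPoints gathers the world transforms of the direct children of ConnectorPoints, so room connections are defined by child components.
; The construction script only calls its parent, and the event graph runs no logic.
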(fn `Get Hall Points`
  (returns (Origin :type "SceneComponent Object Reference") (Next :type "SceneComponent Object Reference"))
  (return (`self.OriginPoint`) (`self.NextPoint`)))

(fn `GetRoomConnectionPoints`
  (returns (`Point Transforms` :type "Array of Transform Structure"))
  (locals (Transforms :type "Array of Transform Structure"))
  (bind _transforms (`local.Transforms`))
  (for _array_element (`SceneComponent.GetChildrenComponents` (`self.ConnectorPoints`) false)
    (`KismetArrayLibrary.Array_Add` _transforms (`SceneComponent.K2_GetComponentToWorld` _array_element)))
  (return _transforms))

(fn `UserConstructionScript`
  (`parent.UserConstructionScript`))