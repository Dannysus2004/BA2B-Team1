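; BP_FurniturePosition is an editor placeholder that previews where furniture sits in the generation setup.
; Its construction script reads the furniture type from the BP_FurnitureDescriptor that its parent component is attached to, then selects a matching preview mesh and colored or wireframe material.
; Without a descriptor, it shows a half-scale red invalid mesh.
; BeginPlay destroys the mesh, so the preview does not appear during play.
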(event `self.ReceiveBeginPlay`
  (`ActorComponent.K2_DestroyComponent` (`self.StaticMesh`)))

(fn `UserConstructionScript`
  (bind _staticmesh (`self.StaticMesh`))
  (bind _asfurniture_descriptor (cast `/Game/Generation/GenerationSetupComponents/BP_FurnitureDescriptor` (`SceneComponent.GetAttachParent` (`self.GetParentComponent`)))
    (:`then`
      (bind _associated_furniture_type (`/Game/Generation/GenerationSetupComponents/BP_FurnitureDescriptor.Associated Furniture Type` _asfurniture_descriptor))
      (`StaticMeshComponent.SetStaticMesh` _staticmesh (select `/Game/Generation/Data/E_FurnitureType` _associated_furniture_type :`NewEnumerator6` "/Game/Generation/DeveloperArt/SM_FurniturePreview_Invalid.SM_FurniturePreview_Invalid" :`NewEnumerator0` "/Game/PLAYTEST/FBXS/SM_BlockOut_RoundTable.SM_BlockOut_RoundTable" :`NewEnumerator1` "/Game/Aimee/Assets/SM_Double_Bed.SM_Double_Bed" :`NewEnumerator2` "/Game/Generation/DeveloperArt/SM_FurniturePreview_WallLight.SM_FurniturePreview_WallLight" :`NewEnumerator3` "/Game/Jake-Asset/JakeAssets/FBXS/SM_Dresser_BLOCK.SM_Dresser_BLOCK" :`NewEnumerator4` "/Game/Generation/DeveloperArt/SM_FurniturePreview_Carpet.SM_FurniturePreview_Carpet" :`NewEnumerator5` "/Game/Aimee/Assets/SM_Chair.SM_Chair" :!type "StaticMesh Object Reference"))
      (`PrimitiveComponent.SetMaterial` _staticmesh 0 (select `/Game/Generation/Data/E_FurnitureType` _associated_furniture_type :`NewEnumerator6` "/Game/Generation/DeveloperArt/MI_FurniturePlaceholder_Red.MI_FurniturePlaceholder_Red" :`NewEnumerator0` "/Game/Generation/DeveloperArt/MI_FurniturePlaceholder_Blue.MI_FurniturePlaceholder_Blue" :`NewEnumerator1` "/Game/Generation/DeveloperArt/MI_FurniturePlaceholder_Red.MI_FurniturePlaceholder_Red" :`NewEnumerator2` "/Game/Generation/DeveloperArt/MI_FurniturePlaceholder_Green.MI_FurniturePlaceholder_Green" :`NewEnumerator3` "/Game/Generation/DeveloperArt/MI_FurniturePlaceholder_Blue.MI_FurniturePlaceholder_Blue" :`NewEnumerator4` "/Game/Generation/DeveloperArt/M_FurniturePlaceholder_Wireframe.M_FurniturePlaceholder_Wireframe" :`NewEnumerator5` "/Game/Generation/DeveloperArt/MI_FurniturePlaceholder_Red.MI_FurniturePlaceholder_Red" :!type "MaterialInterface Object Reference"))
      (`SceneComponent.SetRelativeScale3D` _staticmesh (`KismetMathLibrary.MakeVector` 1.0 1.0 1.0)))
    (:`CastFailed`
      (`StaticMeshComponent.SetStaticMesh` _staticmesh "/Game/Generation/DeveloperArt/SM_FurniturePreview_Invalid.SM_FurniturePreview_Invalid")
      (`PrimitiveComponent.SetMaterial` _staticmesh 0 "/Game/Generation/DeveloperArt/MI_FurniturePlaceholder_Red.MI_FurniturePlaceholder_Red")
      (`SceneComponent.SetRelativeScale3D` _staticmesh (`KismetMathLibrary.MakeVector` 0.5 0.5 0.5)))))