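; BP_RoomSpawnLocation is a placeable spawn-location marker for room generation, tagged with a spawn override of None, InnerRing or OuterRing.
; The construction script shows that override through the GlanceIcon sprite and the Frame's placeholder material.
; BeginPlay destroys the Frame and StaticMesh placeholder components.
; Getters and a setter expose the override and an in-use flag, which records whether the location is taken.
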(event `self.ReceiveBeginPlay`
  (`ActorComponent.K2_DestroyComponent` (`self.Frame`))
  (`ActorComponent.K2_DestroyComponent` (`self.StaticMesh`)))

(fn `GetInUse`
  (returns (Used :type Boolean))
  (return (`self.IsInUse`)))

(fn `GetSpawnOverride`
  (returns (`Override Type` :type "/Game/Generation/Data/E_SpawnOverrideType Enum"))
  (return (`self.SpawnOverrides`)))

(fn `SetInUse`
  (params (Used :type Boolean))
  (set `self.IsInUse` Used))

(fn `UserConstructionScript`
  (bind _spawnoverrides (`self.SpawnOverrides`))
  (`BillboardComponent.SetSprite` (`self.GlanceIcon`) (select `/Game/Generation/Data/E_SpawnOverrideType` _spawnoverrides :`NewEnumerator2` "/Game/Generation/DeveloperArt/T_SpawnLocation_Fallback.T_SpawnLocation_Fallback" :`NewEnumerator0` "/Game/Generation/DeveloperArt/T_SpawnLocation_Inner.T_SpawnLocation_Inner" :`NewEnumerator1` "/Game/Generation/DeveloperArt/T_SpawnLocation_Outer.T_SpawnLocation_Outer" :!type "Texture2D Object Reference"))
  (`PrimitiveComponent.SetMaterial` (`self.Frame`) 0 (select `/Game/Generation/Data/E_SpawnOverrideType` _spawnoverrides :`NewEnumerator2` "/Game/Generation/DeveloperArt/MI_FurniturePlaceholder_Green.MI_FurniturePlaceholder_Green" :`NewEnumerator0` "/Game/Generation/DeveloperArt/MI_DoorframePlaceholder_Wireframe.MI_DoorframePlaceholder_Wireframe" :`NewEnumerator1` "/Game/Generation/DeveloperArt/MI_FurniturePlaceholder_Blue.MI_FurniturePlaceholder_Blue" :!type "MaterialInterface Object Reference")))