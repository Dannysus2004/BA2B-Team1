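; BP_BedroomDoor is a lockable bedroom door that swings open while first-person characters occupy its trigger.
; Overlap events update an occupant list through a server RPC, which triggers client RPCs that play a timeline swing, reversible in direction, with pitch-randomized sound.
; Locking unbinds the overlap events, while the lock's OnRep swaps frame material, toggles door collision and forces the door closed when locked.
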(event `RPC_ClientAnimateDoor`
  (params (Open :type Boolean))
  (bind _dooropenangle (`self.DoorOpenAngle`))
  ;[0.1451 1 0.1373] Client animate door swing
  (`GameplayStatics.PlaySoundAtLocation` (select `bool` Open :`false` "/Game/Charlie/SFX/A_SFX_Door_Close.A_SFX_Door_Close" :`true` "/Game/Charlie/SFX/A_SFX_Door_Open.A_SFX_Door_Open" :!type "SoundBase Object Reference") (`self.K2_GetActorLocation`) (struct) 1.0 (`KismetMathLibrary.RandomFloatInRange` 0.833 1.12) 0.0 null null null null)
  (if Open
    (bind (_direction _angledelta) (`Timeline|DoorOpening` :!label _label)
      (:`Update`
        (`SceneComponent.K2_SetRelativeRotation` (`self.DoorPlaceholder`) (`KismetMathLibrary.MakeRotator` 0.0 0.0 (* _angledelta (`KismetMathLibrary.SelectFloat` (* _dooropenangle -1.0) _dooropenangle (`self.DoorOpensReverse`)))) false false)))
    (else
      (goto _label :!via `Reverse`))))

(event `Set Door Locked Status`
  (params (`Is Locked` :type Boolean))
  ;[0.1451 1 0.1373] Set locked status and bind / unbind events
  (bind _output_get (set `self.bIsLocked` `Is Locked`))
  (if _output_get
    (clear `self.OnActorBeginOverlap`) ; Unbind overlap if locked
    (clear `self.OnActorEndOverlap`)
    (else
      (add `self.OnActorBeginOverlap` (`|CreateDelegate` :!event `Bindable On Begin Overlap`)) ; Bind overlap if unlocked
      (add `self.OnActorEndOverlap` (`|CreateDelegate` :!event `Bindable On End Overlap`)))))

(event `Bindable On Begin Overlap` :!signature `self.OnActorBeginOverlap`
  (params (OverlappedActor :type "Actor Object Reference") (OtherActor :type "Actor Object Reference"))
  ;[0.1451 1 0.1373] Detect when a player actor overlaps the door trigger
  (if (== (`GameplayStatics.GetObjectClass` OtherActor) "/Game/FirstPerson/Blueprints/BP_FirstPersonCharacter.BP_FirstPersonCharacter_C")
    (`self.RPC_ServerOccupancyChanged` OtherActor)))

(event `RPC_ClientOccupancyChanged`
  ;[0.1451 1 0.1373] Client run animation when overlap occupants change
  (`self.RPC_ClientAnimateDoor` (> (`KismetArrayLibrary.Array_Length` (`self.OccupyingPlayers`)) 0)))

(event `Bindable On End Overlap` :!signature `self.OnActorEndOverlap`
  (params (OverlappedActor :type "Actor Object Reference") (OtherActor :type "Actor Object Reference"))
  ;[0.1451 1 0.1373] Detect when a player actor overlaps the door trigger
  (if (== (`GameplayStatics.GetObjectClass` OtherActor) "/Game/FirstPerson/Blueprints/BP_FirstPersonCharacter.BP_FirstPersonCharacter_C")
    (`self.RPC_ServerOccupancyChanged` OtherActor true)))

(event `RPC_ServerOccupancyChanged`
  (params (AffectedOccupant :type "Actor Object Reference") (bEndedOverlap :type Boolean))
  (bind _occupyingplayers (`self.OccupyingPlayers`))
  (if bEndedOverlap
    (`KismetArrayLibrary.Array_RemoveItem` _occupyingplayers AffectedOccupant)
    (else
      (`KismetArrayLibrary.Array_AddUnique` _occupyingplayers AffectedOccupant)))
  (`self.RPC_ClientOccupancyChanged`))

(fn `OnRep_bIsLocked`
  (bind _frame (`self.Frame`))
  (bind _doorplaceholder (`self.DoorPlaceholder`))
  (if (`self.bIsLocked`)
    (`PrimitiveComponent.SetMaterial` _frame 0 "/Game/LevelPrototyping/Materials/MI_Solid_Blue.MI_Solid_Blue")
    (`PrimitiveComponent.SetCollisionEnabled` _doorplaceholder "QueryAndPhysics")
    (`self.RPC_ClientAnimateDoor` false) ; Force close door
    (else
      (`PrimitiveComponent.SetMaterial` _frame 0 "/Game/StarterContent/Materials/M_Metal_Rust.M_Metal_Rust")
      (`PrimitiveComponent.SetCollisionEnabled` _doorplaceholder "NoCollision"))))

(fn `UserConstructionScript`)