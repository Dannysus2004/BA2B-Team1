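; BP_Necronomicon is the Necronomicon object in the game, reporting player proximity and showing particle effects.
; Its Sphere overlap casts to BP_FirstPersonCharacter, stores the reference, and calls NearNecronomiconMessage to flag entering or leaving range, always passing Viable as false.
; NecronomiconPickedUp and NecronomiconActivated events each activate their own Niagara effect.
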(event `self.Sphere.OnComponentBeginOverlap`
  (params (OverlappedComponent :type "PrimitiveComponent Object Reference") (OtherActor :type "Actor Object Reference") (OtherComp :type "PrimitiveComponent Object Reference") (OtherBodyIndex :type Integer) (bFromSweep :type Boolean) (SweepResult :type "HitResult Structure (by ref)"))
  ;[0.06771 0 0.002082] Collision triggered
  (bind _asbp_first_person_character (cast `/Game/FirstPerson/Blueprints/BP_FirstPersonCharacter` OtherActor))
  (bind _output_get (set `self.As BP First Person Character` _asbp_first_person_character))
  (message `/Game/Inez/Sigil/BPI_Collectable.NearNecronomicon` _output_get false true))

(event `self.Sphere.OnComponentEndOverlap`
  (params (OverlappedComponent :type "PrimitiveComponent Object Reference") (OtherActor :type "Actor Object Reference") (OtherComp :type "PrimitiveComponent Object Reference") (OtherBodyIndex :type Integer))
  ;[0.06771 0 0.002082] Collision triggered
  (message `/Game/Inez/Sigil/BPI_Collectable.NearNecronomicon` (`self.As BP First Person Character`) false false))

(event `/Game/Inez/Sigil/BPI_Collectable.NecronomiconPickedUp`
  (`ActorComponent.Activate` (`self.PickedUpNiagara`) false))

(event `/Game/Inez/Sigil/BPI_Collectable.NecronomiconActivated`
  (`ActorComponent.Activate` (`self.ActivatedNiagara`) false))

(fn `UserConstructionScript`)