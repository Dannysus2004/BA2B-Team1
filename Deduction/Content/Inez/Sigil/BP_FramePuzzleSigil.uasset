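; BP_FramePuzzleSigil is a discoverable sigil that becomes detectable by the player once its frame puzzle is complete.
; Sphere overlaps message the first-person character with proximity, active state and a trace collision reference, gated by PuzzleComplete.
; SigilFound deactivates the sigil and plays discovery feedback through sound, light, decal material and Niagara.
; An unconnected node would unhide four corner components.
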(event `self.Sphere.OnComponentBeginOverlap`
  (params (OverlappedComponent :type "PrimitiveComponent Object Reference") (OtherActor :type "Actor Object Reference") (OtherComp :type "PrimitiveComponent Object Reference") (OtherBodyIndex :type Integer) (bFromSweep :type Boolean) (SweepResult :type "HitResult Structure (by ref)"))
  ;[0.05448 0 0] Sends collided state to overlapping player
  (if (`self.PuzzleComplete`)
    (bind _asbp_first_person_character (cast `/Game/FirstPerson/Blueprints/BP_FirstPersonCharacter` OtherActor))
    (bind _output_get (set `self.As BP First Person Character` _asbp_first_person_character))
    (message `/Game/Inez/Sigil/BPI_Collectable.NearSigil` _output_get true (`self.Active`) (`self.TraceCollison`))))

(event `self.Sphere.OnComponentEndOverlap`
  (params (OverlappedComponent :type "PrimitiveComponent Object Reference") (OtherActor :type "Actor Object Reference") (OtherComp :type "PrimitiveComponent Object Reference") (OtherBodyIndex :type Integer))
  ;[0.05448 0 0] Sends collided state to overlapping player
  (if (`self.PuzzleComplete`)
    (message `/Game/Inez/Sigil/BPI_Collectable.NearSigil` (`self.As BP First Person Character`) false false null)))

(event `self.SigilFound`
  ;[0.05448 0 0] Sigil reaction to being discovered
  (set `self.Active` false)
  (`GameplayStatics.PlaySoundAtLocation` "/Game/Inez/Sigil/Audio/SC_Bong.SC_Bong" (`self.K2_GetActorLocation`) (struct) 1.0 1.0 0.0 null null null null)
  (`LightComponent.SetIntensity` (`self.PointLight`) 5000.0)
  (`DecalComponent.SetDecalMaterial` (`self.Decal`) "/Game/Inez/Sigil/Decals/DM_SigilEmisivePlaceholder1.DM_SigilEmisivePlaceholder1")
  (`ActorComponent.SetActive` (`self.Niagara`) true false)
  (`ActorComponent.Activate` (`self.Audio`) false))

(fn `UserConstructionScript`)